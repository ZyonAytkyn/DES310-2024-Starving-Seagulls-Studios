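; BP_CameraMan is a camera manager that switches the player's view between fixed scene cameras for puzzles, a clock close-up, the grand entrance and character groups.
; It exposes one function per shot, each finding the first actor with a matching tag and passing it to player controller 0's SetViewTargetWithBlend.
; Cameras are located by tag lookup on every call, with no stored references or check for a missing camera.
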(event `self.ReceiveBeginPlay`)

(fn `ChangeToBookcasePuzzleCamera`
  (bind _outactors (`GameplayStatics.GetAllActorsWithTag` "BookcasePuzzleCamera"))
  (`PlayerController.SetViewTargetWithBlend` (`GameplayStatics.GetPlayerController` 0) (`|GetArrayItem` _outactors) 0.0 "VTBlend_Linear" 0.0 false))

(fn `ChangeToClockCloseupCamera`
  (bind _outactors (`GameplayStatics.GetAllActorsWithTag` "ClockCloseupCamera"))
  (`PlayerController.SetViewTargetWithBlend` (`GameplayStatics.GetPlayerController` 0) (`|GetArrayItem` _outactors) 0.0 "VTBlend_Linear" 0.0 false))

(fn `ChangeToFlappersCamera`
  (bind _outactors (`GameplayStatics.GetAllActorsWithTag` "FlappersCamera"))
  (`PlayerController.SetViewTargetWithBlend` (`GameplayStatics.GetPlayerController` 0) (`|GetArrayItem` _outactors) 0.0 "VTBlend_Linear" 0.0 false))

(fn `ChangeToGangsterCamera`
  (bind _outactors (`GameplayStatics.GetAllActorsWithTag` "GangsterCamera"))
  (`PlayerController.SetViewTargetWithBlend` (`GameplayStatics.GetPlayerController` 0) (`|GetArrayItem` _outactors) 0.0 "VTBlend_Linear" 0.0 false))

(fn `ChangeToGrandEnteranceCamera`
  (bind _outactors (`GameplayStatics.GetAllActorsWithTag` "GrandEnteranceCamera"))
  (`PlayerController.SetViewTargetWithBlend` (`GameplayStatics.GetPlayerController` 0) (`|GetArrayItem` _outactors) 0.0 "VTBlend_Linear" 0.0 false))

(fn `ChangeToJigsawPuzzleCamera`
  (bind _outactors (`GameplayStatics.GetAllActorsWithTag` "JigsawPuzzleCamera"))
  (`PlayerController.SetViewTargetWithBlend` (`GameplayStatics.GetPlayerController` 0) (`|GetArrayItem` _outactors) 0.0 "VTBlend_Linear" 0.0 false))

(fn `ChangeToRichCoupleCamera`
  (bind _outactors (`GameplayStatics.GetAllActorsWithTag` "RichCoupleCamera"))
  (`PlayerController.SetViewTargetWithBlend` (`GameplayStatics.GetPlayerController` 0) (`|GetArrayItem` _outactors) 0.0 "VTBlend_Linear" 0.0 false))

(fn `ChangeToSafePuzzleCamera`
  (bind _outactors (`GameplayStatics.GetAllActorsWithTag` "SafePuzzleCamera"))
  (`PlayerController.SetViewTargetWithBlend` (`GameplayStatics.GetPlayerController` 0) (`|GetArrayItem` _outactors) 0.0 "VTBlend_Linear" 0.0 false))

(fn `UserConstructionScript`)