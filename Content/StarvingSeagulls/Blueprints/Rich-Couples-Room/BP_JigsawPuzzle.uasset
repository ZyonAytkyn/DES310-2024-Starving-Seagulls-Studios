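; Drag-and-drop nine-piece jigsaw puzzle actor for the rich couple's room.
; Clicked pieces follow the cursor trace hit on Tick using hard-coded offsets, freeing their slot when lifted.
; On release, pieces snap to nearby free slots in CorrectPositions; once all slots fill, each piece is checked against its correct index.
; A correct solution updates HUD and room widgets and returns the view to the room camera.
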(event `self.ReceiveBeginPlay`
  (bind _allpieces (`self.AllPieces`))
  (`KismetArrayLibrary.Array_Add` _allpieces (`self.Test`))
  (`KismetArrayLibrary.Array_Add` _allpieces (`self.Test1`))
  (`KismetArrayLibrary.Array_Add` _allpieces (`self.Test2`))
  (`KismetArrayLibrary.Array_Add` _allpieces (`self.Test3`))
  (`KismetArrayLibrary.Array_Add` _allpieces (`self.Test4`))
  (`KismetArrayLibrary.Array_Add` _allpieces (`self.Test5`))
  (`KismetArrayLibrary.Array_Add` _allpieces (`self.Test6`))
  (`KismetArrayLibrary.Array_Add` _allpieces (`self.Test7`))
  (`KismetArrayLibrary.Array_Add` _allpieces (`self.Test8`))
  (`WidgetBlueprintLibrary.SetInputMode_GameAndUIEx` (`GameplayStatics.GetPlayerController` 0) null "DoNotLock" false))

(event `self.ReceiveTick`
  (params (DeltaSeconds :type "Float (single-precision)"))
  (bind _hitpiece (`self.HitPiece`))
  (bind _hitresult (`PlayerController.GetHitResultUnderCursorForObjects` (`GameplayStatics.GetPlayerController` 0) (`|MakeArray` "ObjectTypeQuery2" :!type "EObjectTypeQuery Enum") true))
  (`KismetSystemLibrary.PrintString` (`KismetStringLibrary.Conv_DoubleToString` (.x (`.Location` (`GameplayStatics.BreakHitResult` _hitresult)))) false false (struct :`R` 1.0 :`B` 0.299861 :`A` 1.0))
  (`KismetSystemLibrary.PrintString` (`KismetStringLibrary.Conv_DoubleToString` (.z (`.Location` (`GameplayStatics.BreakHitResult` _hitresult)))) false false (struct :`G` 0.068355 :`B` 1.0 :`A` 1.0))
  (if (`self.PieceSelected`)
    (`WidgetLayoutLibrary.GetMousePositionOnPlatform`)
    (`SceneComponent.K2_SetRelativeLocation` _hitpiece (`KismetMathLibrary.MakeVector` (- (.x (`.Location` (`GameplayStatics.BreakHitResult` _hitresult))) 9200.0) 0.5 (- (.z (`.Location` (`GameplayStatics.BreakHitResult` _hitresult))) 1480.0)) false false)
    (`KismetSystemLibrary.PrintString` (`KismetStringLibrary.Conv_VectorToString` (`SceneComponent.RelativeLocation` _hitpiece)) false false)))

(event `self.Test.OnClicked`
  (params (TouchedComponent :type "PrimitiveComponent Object Reference") (ButtonPressed :type "Key Structure"))
  (set `self.HitPiece` (`.HitComponent` (`GameplayStatics.BreakHitResult` (`PlayerController.GetHitResultUnderCursorForObjects` (`GameplayStatics.GetPlayerController` 0) (`|MakeArray` "ObjectTypeQuery2" :!type "EObjectTypeQuery Enum") true))) :!label _label)
  (`GameplayStatics.PlaySound2D` "/Game/StarvingSeagulls/Blueprints/Flappers-Room/FlapperSounds/560700__el_boss__puzzle-piece-rotation-clockwise.560700__el_boss__puzzle-piece-rotation-clockwise" 1.0 1.0 0.0 null null)
  (`self.IsPiecePlaced`)
  (set `self.PieceSelected` true))

(event `self.Test1.OnClicked`
  (params (TouchedComponent :type "PrimitiveComponent Object Reference") (ButtonPressed :type "Key Structure"))
  (goto _label))

(event `self.Test.OnReleased`
  (params (TouchedComponent :type "PrimitiveComponent Object Reference") (ButtonReleased :type "Key Structure"))
  (set `self.PieceSelected` false :!label _label_2)
  (`GameplayStatics.PlaySound2D` "/Game/StarvingSeagulls/Blueprints/Flappers-Room/FlapperSounds/546119__el_boss__piece-placement.546119__el_boss__piece-placement" 1.0 1.0 0.0 null null)
  (`self.FindClosestPosition`)
  (`self.IsAllPiecesPlaced`)
  (if (`self.AllPlaced`)
    (`self.SolutionChecker`)
    (if (`self.IsSolutionCorrect`)
      (`self.PuzzleCompleted`))))

(event `self.Test2.OnClicked`
  (params (TouchedComponent :type "PrimitiveComponent Object Reference") (ButtonPressed :type "Key Structure"))
  (goto _label))

(event `self.Test1.OnReleased`
  (params (TouchedComponent :type "PrimitiveComponent Object Reference") (ButtonReleased :type "Key Structure"))
  (goto _label_2))

(event `self.Test3.OnClicked`
  (params (TouchedComponent :type "PrimitiveComponent Object Reference") (ButtonPressed :type "Key Structure"))
  (goto _label))

(event `self.Test2.OnReleased`
  (params (TouchedComponent :type "PrimitiveComponent Object Reference") (ButtonReleased :type "Key Structure"))
  (goto _label_2))

(event `self.Test4.OnClicked`
  (params (TouchedComponent :type "PrimitiveComponent Object Reference") (ButtonPressed :type "Key Structure"))
  (goto _label))

(event `PuzzleCompleted`
  (bind _foundwidgets (`WidgetBlueprintLibrary.GetAllWidgetsOfClass` "/Game/StarvingSeagulls/UI/LevelUI/InGameHUD.InGameHUD_C" false))
  (`/Game/StarvingSeagulls/UI/LevelUI/InGameHUD.SetToNotPuzzle` (`|GetArrayItem` _foundwidgets))
  (bind _foundwidgets_2 (`WidgetBlueprintLibrary.GetAllWidgetsOfClass` "/Game/StarvingSeagulls/UI/LevelUI/RichCoupleRoom.RichCoupleRoom_C" false))
  (`/Game/StarvingSeagulls/UI/LevelUI/RichCoupleRoom.JigsawPuzzleCompleted` (`|GetArrayItem` _foundwidgets_2))
  (bind _outactors (`GameplayStatics.GetAllActorsOfClassWithTag` "/Script/Engine.CameraActor" "RichCoupleCamera"))
  (`PlayerController.SetViewTargetWithBlend` (`GameplayStatics.GetPlayerController` 0) (`|GetArrayItem` _outactors) 0.0 "VTBlend_Linear" 0.0 false)
  (bind _foundwidgets_3 (`WidgetBlueprintLibrary.GetAllWidgetsOfClass` "/Game/StarvingSeagulls/UI/LevelUI/FlapperRoomClickables.FlapperRoomClickables_C" false))
  (set `/Game/StarvingSeagulls/UI/LevelUI/FlapperRoomClickables.PuzzleActive` false (`|GetArrayItem` _foundwidgets_3)))

(event `self.Test3.OnReleased`
  (params (TouchedComponent :type "PrimitiveComponent Object Reference") (ButtonReleased :type "Key Structure"))
  (goto _label_2))

(event `self.Test5.OnClicked`
  (params (TouchedComponent :type "PrimitiveComponent Object Reference") (ButtonPressed :type "Key Structure"))
  (goto _label))

(event `self.Test4.OnReleased`
  (params (TouchedComponent :type "PrimitiveComponent Object Reference") (ButtonReleased :type "Key Structure"))
  (goto _label_2))

(event `self.Test6.OnClicked`
  (params (TouchedComponent :type "PrimitiveComponent Object Reference") (ButtonPressed :type "Key Structure"))
  (goto _label))

(event `self.Test5.OnReleased`
  (params (TouchedComponent :type "PrimitiveComponent Object Reference") (ButtonReleased :type "Key Structure"))
  (goto _label_2))

(event `self.Test7.OnClicked`
  (params (TouchedComponent :type "PrimitiveComponent Object Reference") (ButtonPressed :type "Key Structure"))
  (goto _label))

(event `self.Test6.OnReleased`
  (params (TouchedComponent :type "PrimitiveComponent Object Reference") (ButtonReleased :type "Key Structure"))
  (goto _label_2))

(event `self.Test8.OnClicked`
  (params (TouchedComponent :type "PrimitiveComponent Object Reference") (ButtonPressed :type "Key Structure"))
  (goto _label))

(event `self.Test7.OnReleased`
  (params (TouchedComponent :type "PrimitiveComponent Object Reference") (ButtonReleased :type "Key Structure"))
  (goto _label_2))

(event `self.Stop.OnClicked`
  (params (TouchedComponent :type "PrimitiveComponent Object Reference") (ButtonPressed :type "Key Structure"))
  ;[1 1 1] used for testing
)

(event `self.Test8.OnReleased`
  (params (TouchedComponent :type "PrimitiveComponent Object Reference") (ButtonReleased :type "Key Structure"))
  (goto _label_2))

(fn `FindClosestPosition`
  (for (_array_element _array_index) (`self.CorrectPositions`)
    (if (and (< (`KismetMathLibrary.Vector_Distance` _array_element (`SceneComponent.RelativeLocation` (`self.HitPiece`))) 30.0) (`|GetArrayItem` (`self.PositonAvailable`) _array_index))
      (`SceneComponent.K2_SetRelativeLocation` (`self.HitPiece`) _array_element false false)
      (`KismetArrayLibrary.Array_Set` (`self.PositonAvailable`) _array_index)
      (break))))

(fn `IsAllPiecesPlaced`
  (set `self.AllPlaced` true)
  (for _array_element (`self.PositonAvailable`)
    (if _array_element
      (set `self.AllPlaced` false)
      (break))))

(fn `IsPiecePlaced`
  (for (_array_element _array_index) (`self.CorrectPositions`)
    (if (== (`SceneComponent.RelativeLocation` (`self.HitPiece`)) _array_element :`ErrorTolerance` 1.0)
      (`KismetArrayLibrary.Array_Set` (`self.PositonAvailable`) _array_index true)
      (break))))

(fn `SolutionChecker`
  (set `self.IsSolutionCorrect` true)
  (for (_ _array_index) (`self.AllPieces`)
    (if (not (== (`|GetArrayItem` (`self.CorrectPositions`) (`|GetArrayItem` (`self.CorrectPieceIndex`) _array_index)) (`SceneComponent.RelativeLocation` (`|GetArrayItem` (`self.AllPieces`) _array_index)) :`ErrorTolerance` 1.0))
      (set `self.IsSolutionCorrect` false))))

(fn `UserConstructionScript`)