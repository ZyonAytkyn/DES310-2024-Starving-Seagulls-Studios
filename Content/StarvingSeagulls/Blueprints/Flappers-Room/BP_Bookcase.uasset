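; Bookcase puzzle actor for the Flapper room, solved by arranging clickable books in the correct order on the top shelf.
; Clicking a book shows its cover and two markers: the first empty slot or its original position.
; Each placement updates PlacementOrder, whose trimmed copy SolutionChecker compares to TheCorrectSolution.
; A match updates the HUD and room widget and returns to FlapperCamera; older click-sequence logic remains unwired.
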(event `self.Book P.OnClicked`
  (params (TouchedComponent :type "PrimitiveComponent Object Reference") (ButtonPressed :type "Key Structure"))
  ;[1 1 1] More Old Stuff
)

(event `self.Book C.OnClicked`
  (params (TouchedComponent :type "PrimitiveComponent Object Reference") (ButtonPressed :type "Key Structure"))
  ;[1 1 1] More Old Stuff
)

(event `self.SpriteBook P.OnClicked`
  (params (TouchedComponent :type "PrimitiveComponent Object Reference") (ButtonPressed :type "Key Structure"))
  (`GameplayStatics.PlaySound2D` "/Game/StarvingSeagulls/Blueprints/Flappers-Room/FlapperSounds/667384__mastersuite__book-pullout.667384__mastersuite__book-pullout" 1.0 1.0 0.0 null null)
  (`self.OnBookClicked` (`self.SpriteBook P`) 5))

(event `self.SpriteBook H.OnClicked`
  (params (TouchedComponent :type "PrimitiveComponent Object Reference") (ButtonPressed :type "Key Structure"))
  (`GameplayStatics.PlaySound2D` "/Game/StarvingSeagulls/Blueprints/Flappers-Room/FlapperSounds/667384__mastersuite__book-pullout.667384__mastersuite__book-pullout" 1.0 1.0 0.0 null null)
  (`self.OnBookClicked` (`self.SpriteBook H`) 7))

(event `self.Book U.OnClicked`
  (params (TouchedComponent :type "PrimitiveComponent Object Reference") (ButtonPressed :type "Key Structure"))
  ;[1 1 1] More Old Stuff
)

(event `self.Book E.OnClicked`
  (params (TouchedComponent :type "PrimitiveComponent Object Reference") (ButtonPressed :type "Key Structure"))
  ;[1 1 1] More Old Stuff
)

(event `self.SpriteBook U.OnClicked`
  (params (TouchedComponent :type "PrimitiveComponent Object Reference") (ButtonPressed :type "Key Structure"))
  (`GameplayStatics.PlaySound2D` "/Game/StarvingSeagulls/Blueprints/Flappers-Room/FlapperSounds/667384__mastersuite__book-pullout.667384__mastersuite__book-pullout" 1.0 1.0 0.0 null null)
  (`self.OnBookClicked` (`self.SpriteBook U`) 1))

(event `self.SpriteBook E.OnClicked`
  (params (TouchedComponent :type "PrimitiveComponent Object Reference") (ButtonPressed :type "Key Structure"))
  (`GameplayStatics.PlaySound2D` "/Game/StarvingSeagulls/Blueprints/Flappers-Room/FlapperSounds/667384__mastersuite__book-pullout.667384__mastersuite__book-pullout" 1.0 1.0 0.0 null null)
  (`self.OnBookClicked` (`self.SpriteBook E`)))

(event `self.Book N.OnClicked`
  (params (TouchedComponent :type "PrimitiveComponent Object Reference") (ButtonPressed :type "Key Structure"))
  ;[1 1 1] More Old Stuff
)

(event `self.Book O.OnClicked`
  (params (TouchedComponent :type "PrimitiveComponent Object Reference") (ButtonPressed :type "Key Structure"))
  ;[1 1 1] More Old Stuff
)

(event `self.SpriteBook N.OnClicked`
  (params (TouchedComponent :type "PrimitiveComponent Object Reference") (ButtonPressed :type "Key Structure"))
  (`GameplayStatics.PlaySound2D` "/Game/StarvingSeagulls/Blueprints/Flappers-Room/FlapperSounds/667384__mastersuite__book-pullout.667384__mastersuite__book-pullout" 1.0 1.0 0.0 null null)
  (`self.OnBookClicked` (`self.SpriteBook N`) 3))

(event `self.SpriteBook L.OnClicked`
  (params (TouchedComponent :type "PrimitiveComponent Object Reference") (ButtonPressed :type "Key Structure"))
  (`GameplayStatics.PlaySound2D` "/Game/StarvingSeagulls/Blueprints/Flappers-Room/FlapperSounds/667384__mastersuite__book-pullout.667384__mastersuite__book-pullout" 1.0 1.0 0.0 null null)
  (`self.OnBookClicked` (`self.SpriteBook L`) 6))

(event `self.Book Z.OnClicked`
  (params (TouchedComponent :type "PrimitiveComponent Object Reference") (ButtonPressed :type "Key Structure"))
  ;[1 1 1] More Old Stuff
)

(event `self.Book H.OnClicked`
  (params (TouchedComponent :type "PrimitiveComponent Object Reference") (ButtonPressed :type "Key Structure"))
  ;[1 1 1] More Old Stuff
)

(event `self.SpriteBook C.OnClicked`
  (params (TouchedComponent :type "PrimitiveComponent Object Reference") (ButtonPressed :type "Key Structure"))
  (`GameplayStatics.PlaySound2D` "/Game/StarvingSeagulls/Blueprints/Flappers-Room/FlapperSounds/667384__mastersuite__book-pullout.667384__mastersuite__book-pullout" 1.0 1.0 0.0 null null)
  (`self.OnBookClicked` (`self.SpriteBook C`) 2))

(event `self.SpriteBook A.OnClicked`
  (params (TouchedComponent :type "PrimitiveComponent Object Reference") (ButtonPressed :type "Key Structure"))
  (`GameplayStatics.PlaySound2D` "/Game/StarvingSeagulls/Blueprints/Flappers-Room/FlapperSounds/667384__mastersuite__book-pullout.667384__mastersuite__book-pullout" 1.0 1.0 0.0 null null)
  (`self.OnBookClicked` (`self.SpriteBook A`) 4))

(event `self.RoomCube.OnClicked`
  (params (TouchedComponent :type "PrimitiveComponent Object Reference") (ButtonPressed :type "Key Structure"))
  ;[1 1 1] Just for play party
)

(event `FullPuzzleReset`
  ;[1 1 1] NO
  ;;[1 0 0] Full Puzzle Reset
)

(event `self.ReceiveBeginPlay`
  ;[1 1 1] Just for play party
)

(event `PuzzleCompleted`
  ;[0 1 0] Puzzle Complete
  (bind _foundwidgets (`WidgetBlueprintLibrary.GetAllWidgetsOfClass` "/Game/StarvingSeagulls/UI/LevelUI/InGameHUD.InGameHUD_C" false))
  (`/Game/StarvingSeagulls/UI/LevelUI/InGameHUD.SetToNotPuzzle` (`|GetArrayItem` _foundwidgets))
  (bind _foundwidgets_2 (`WidgetBlueprintLibrary.GetAllWidgetsOfClass` "/Game/StarvingSeagulls/UI/LevelUI/FlapperRoomClickables.FlapperRoomClickables_C" false))
  (`/Game/StarvingSeagulls/UI/LevelUI/FlapperRoomClickables.BookcasePuzzleCompleted` (`|GetArrayItem` _foundwidgets_2))
  (bind _outactors (`GameplayStatics.GetAllActorsOfClassWithTag` "/Script/Engine.CameraActor" "FlapperCamera"))
  (`PlayerController.SetViewTargetWithBlend` (`GameplayStatics.GetPlayerController` 0) (`|GetArrayItem` _outactors) 0.0 "VTBlend_Linear" 0.0 false)
  (bind _foundwidgets_3 (`WidgetBlueprintLibrary.GetAllWidgetsOfClass` "/Game/StarvingSeagulls/UI/LevelUI/FlapperRoomClickables.FlapperRoomClickables_C" false))
  (set `/Game/StarvingSeagulls/UI/LevelUI/FlapperRoomClickables.PuzzleActive` false (`|GetArrayItem` _foundwidgets_3)))

(event `self.ReceiveTick`
  (params (DeltaSeconds :type "Float (single-precision)"))
  ;[1 1 1] Print Placement Order
)

(event `self.Available Placement.OnClicked`
  (params (TouchedComponent :type "PrimitiveComponent Object Reference") (ButtonPressed :type "Key Structure"))
  ;[1 1 1] When Placed on top shelf
  (if (`self.BookHasBeenClicked`)
    (`self.OnBookPlaced` (`self.SelectedBook`) (`self.NumberOfOriginalBookPlacement`))
    (`GameplayStatics.PlaySound2D` "/Game/StarvingSeagulls/Blueprints/Flappers-Room/FlapperSounds/667385__mastersuite__book-pushin.667385__mastersuite__book-pushin" 1.0 1.0 0.0 null null)
    (`self.SolutionChecker`)))

(event `self.Original Placement.OnClicked`
  (params (TouchedComponent :type "PrimitiveComponent Object Reference") (ButtonPressed :type "Key Structure"))
  ;[1 1 1] When Returned to Orignal Position
  (if (`self.BookHasBeenClicked`)
    (`self.OnBookReturned` (`self.SelectedBook`))
    (`GameplayStatics.PlaySound2D` "/Game/StarvingSeagulls/Blueprints/Flappers-Room/FlapperSounds/667385__mastersuite__book-pushin.667385__mastersuite__book-pushin" 1.0 1.0 0.0 null null)))

(fn `OnBookClicked`
  (params (SpriteBook :type "PaperSpriteComponent Object Reference") (OriginalBookPlacementNum :type Integer) (Book :type "PrimitiveComponent Object Reference"))
  (bind _placementorder (`self.PlacementOrder`))
  (bind _loopnum (`self.LoopNum`))
  (bind _available_placement (`self.Available Placement`))
  (bind _original_placement (`self.Original Placement`))
  (bind _coverview (`self.CoverView`))
  (bind _numberoforiginalbookplacement (`self.NumberOfOriginalBookPlacement`))
  (bind _returnvalue (`KismetArrayLibrary.Array_Find` (`self.PlacementOrder`) (`self.Empty Space`)))
  (bind _returnvalue_2 (`KismetArrayLibrary.Array_Find` (`self.PlacementOrder`) (`self.NumberOfOriginalBookPlacement`)))
  (bind (_output_x _output_y _output_z) (`KismetMathLibrary.BreakVector` (`|GetArrayItem` (`self.OriginalBookLocations`) _numberoforiginalbookplacement)))
  (if (not (`self.BookHasBeenClicked`))
    (set `self.NumberOfOriginalBookPlacement` OriginalBookPlacementNum)
    (if (!= _returnvalue_2 -1)
      (`KismetArrayLibrary.Array_Set` (`self.PlacementOrder`) _returnvalue_2 (`self.Empty Space`))
      (set `self.NumberOfPlacedBooks` 0)
      (for _array_element _placementorder
        (if (== _array_element 99)
          (`/Engine/EditorBlueprintResources/StandardMacros.IncrementInt` _loopnum
            (:`  `
              _))
          (else
            (`/Engine/EditorBlueprintResources/StandardMacros.IncrementInt` (`self.NumberOfPlacedBooks`)
              (:`  `
                (`/Engine/EditorBlueprintResources/StandardMacros.IncrementInt` _loopnum
                  (:`  `
                    _))))))
        (if (>= _loopnum (`KismetArrayLibrary.Array_Length` _placementorder))
          (break))))
    (set `self.SelectedBook` SpriteBook)
    (`SceneComponent.SetHiddenInGame` SpriteBook true true)
    (`SceneComponent.K2_SetRelativeLocation` SpriteBook (0.0 -200.0 0.0) false false)
    (set `self.BookPlacementIndex` _returnvalue)
    (`SceneComponent.K2_SetRelativeLocation` _available_placement (`|GetArrayItem` (`self.BookPlacementLocations`) _returnvalue) false false)
    (`SceneComponent.K2_SetRelativeLocation` _original_placement (`KismetMathLibrary.MakeVector` _output_x -5.0 _output_z) false false)
    (`PaperSpriteComponent.SetSprite` _coverview (`|GetArrayItem` (`self.Book Covers`) _numberoforiginalbookplacement))
    (`SceneComponent.SetHiddenInGame` _coverview false false)
    (`SceneComponent.SetHiddenInGame` _available_placement false false)
    (`SceneComponent.SetHiddenInGame` _original_placement false false)
    (set `self.BookHasBeenClicked` true)))

(fn `OnBookPlaced`
  (params (SpriteBook :type "PaperSpriteComponent Object Reference") (OriginalBookPlacementNum :type Integer) (Book :type "PrimitiveComponent Object Reference"))
  (bind _available_placement (`self.Available Placement`))
  (bind _available_placement_2 (`self.Available Placement`))
  (`KismetArrayLibrary.Array_Set` (`self.PlacementOrder`) (`self.BookPlacementIndex`) OriginalBookPlacementNum)
  (`SceneComponent.K2_SetRelativeTransform` SpriteBook (`KismetMathLibrary.MakeTransform` (`SceneComponent.RelativeLocation` _available_placement) (`SceneComponent.RelativeRotation` _available_placement) (`SceneComponent.RelativeScale3D` SpriteBook)) false false)
  (`SceneComponent.SetHiddenInGame` (`self.Original Placement`) true false)
  (`SceneComponent.SetHiddenInGame` _available_placement_2 true false)
  (`SceneComponent.SetHiddenInGame` SpriteBook false true)
  (`SceneComponent.K2_SetRelativeLocation` _available_placement_2 (- (`SceneComponent.RelativeLocation` _available_placement_2) (100.0 0.0 0.0)) false false)
  (`SceneComponent.SetHiddenInGame` (`self.CoverView`) true false)
  (if (< (`KismetArrayLibrary.Array_Find` (`self.PlacementOrder`) (`self.NumberOfOriginalBookPlacement`)) 98)
    (`/Engine/EditorBlueprintResources/StandardMacros.IncrementInt` (`self.NumberOfPlacedBooks`)
      (:`  `
        _)))
  (set `self.BookHasBeenClicked` false))

(fn `OnBookReturned`
  (params (SpriteBook :type "PaperSpriteComponent Object Reference") (Book :type "PrimitiveComponent Object Reference"))
  (bind _original_placement (`self.Original Placement`))
  (bind _original_placement_2 (`self.Original Placement`))
  (bind (_relativelocation_x _relativelocation_y _relativelocation_z) (`KismetMathLibrary.BreakVector` (`SceneComponent.RelativeLocation` _original_placement)))
  (`SceneComponent.K2_SetRelativeTransform` SpriteBook (`KismetMathLibrary.MakeTransform` (`KismetMathLibrary.MakeVector` _relativelocation_x -10.0 _relativelocation_z) (`SceneComponent.RelativeRotation` _original_placement) (`SceneComponent.RelativeScale3D` SpriteBook)) false false)
  (`SceneComponent.SetHiddenInGame` _original_placement_2 true false)
  (`SceneComponent.SetHiddenInGame` (`self.Available Placement`) true false)
  (`SceneComponent.K2_SetRelativeLocation` _original_placement_2 (- (`SceneComponent.RelativeLocation` _original_placement_2) (100.0 0.0 0.0)) false false)
  (`SceneComponent.SetHiddenInGame` SpriteBook false true)
  (`SceneComponent.SetHiddenInGame` (`self.CoverView`) true false)
  (set `self.BookHasBeenClicked` false))

(fn `ResetMaterial`
  (`PrimitiveComponent.SetMaterial` (`self.Book P`) 0 "/Game/StarterContent/Materials/M_Basic_Wall.M_Basic_Wall")
  (`PrimitiveComponent.SetMaterial` (`self.Book U`) 0 "/Game/StarterContent/Materials/M_Basic_Wall.M_Basic_Wall")
  (`PrimitiveComponent.SetMaterial` (`self.Book N`) 0 "/Game/StarterContent/Materials/M_Basic_Wall.M_Basic_Wall")
  (`PrimitiveComponent.SetMaterial` (`self.Book C`) 0 "/Game/StarterContent/Materials/M_Basic_Wall.M_Basic_Wall")
  (`PrimitiveComponent.SetMaterial` (`self.Book H`) 0 "/Game/StarterContent/Materials/M_Basic_Wall.M_Basic_Wall"))

(fn `ResetPuzzle`
  (set `self.ClickedBookP` false)
  (set `self.ClickedBookU` false)
  (set `self.ClickedBookN` false)
  (set `self.ClickedBookC` false))

(fn `SetMaterial`
  (params (Book :type "PrimitiveComponent Object Reference"))
  (`PrimitiveComponent.SetMaterial` Book 0 "/Game/StarterContent/Materials/M_Metal_Gold.M_Metal_Gold"))

(fn `SolutionChecker`
  (bind _shrunksolutioncheckarray (`self.ShrunkSolutionCheckArray`))
  (set `self.ShrunkSolutionCheckArray` (`self.PlacementOrder`))
  (`KismetArrayLibrary.Array_Remove` _shrunksolutioncheckarray 7)
  (`KismetArrayLibrary.Array_Remove` _shrunksolutioncheckarray 6)
  (`KismetArrayLibrary.Array_Remove` _shrunksolutioncheckarray 5)
  (if (`KismetArrayLibrary.Array_Identical` _shrunksolutioncheckarray (`self.TheCorrectSolution`))
    (`self.PuzzleCompleted`)))

(fn `UserConstructionScript`
  (`SceneComponent.SetHiddenInGame` (`self.Available Placement`) true false)
  (`SceneComponent.SetHiddenInGame` (`self.Original Placement`) true false)
  (`SceneComponent.SetHiddenInGame` (`self.SolvedText`) true false))