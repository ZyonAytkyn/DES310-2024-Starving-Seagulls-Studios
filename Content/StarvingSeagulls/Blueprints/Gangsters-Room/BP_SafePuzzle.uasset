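; Three-dial safe combination puzzle in the Gangster's Room whose solution triggers the game's ending.
; Clickable up and down components step each dial from 0 to 11 with wraparound, updating its number sprite.
; After every click, SolutionChecker compares the dial values to the Solution array.
; A match runs SafePuzzleComplete, a timed sequence that hides HUD elements, switches tagged cameras, plays the safe-opening media and loads EndGameLevel.
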(event `self.ReceiveBeginPlay`)

(event `self.FirstUp.OnClicked`
  (params (TouchedComponent :type "PrimitiveComponent Object Reference") (ButtonPressed :type "Key Structure"))
  (bind _firstlock (`self.FirstLock`))
  (`GameplayStatics.PlaySound2D` "/Game/StarvingSeagulls/Blueprints/Flappers-Room/FlapperSounds/41506__digifishmusic__knife_sharpen_click.41506__digifishmusic__knife_sharpen_click" 1.0 1.0 0.0 null null)
  (if (< (`self.FirstLockValue`) 11)
    (`self.IncreaseValue` _firstlock)
    (else
      (`self.SetValueZero` _firstlock)))
  (`self.SolutionChecker` :!label _label))

(event `self.FirstDown.OnClicked`
  (params (TouchedComponent :type "PrimitiveComponent Object Reference") (ButtonPressed :type "Key Structure"))
  (bind _firstlock (`self.FirstLock`))
  (`GameplayStatics.PlaySound2D` "/Game/StarvingSeagulls/Blueprints/Flappers-Room/FlapperSounds/41506__digifishmusic__knife_sharpen_click.41506__digifishmusic__knife_sharpen_click" 1.0 1.0 0.0 null null)
  (if (> (`self.FirstLockValue`) 0)
    (`self.DecreaseValue` _firstlock)
    (goto _label)
    (else
      (`self.SetValueEleven` _firstlock)
      (goto _label))))

(event `self.SecondUp.OnClicked`
  (params (TouchedComponent :type "PrimitiveComponent Object Reference") (ButtonPressed :type "Key Structure"))
  (bind _secondlock (`self.SecondLock`))
  (`GameplayStatics.PlaySound2D` "/Game/StarvingSeagulls/Blueprints/Flappers-Room/FlapperSounds/41506__digifishmusic__knife_sharpen_click.41506__digifishmusic__knife_sharpen_click" 1.0 1.0 0.0 null null)
  (if (< (`self.SecondLockValue`) 11)
    (`self.IncreaseValue` _secondlock)
    (goto _label)
    (else
      (`self.SetValueZero` _secondlock)
      (goto _label))))

(event `SafePuzzleComplete`
  (`GameplayStatics.PlaySound2D` "/Game/StarvingSeagulls/Blueprints/Flappers-Room/FlapperSounds/495674__jack_urbanski__vibraphone-chord.495674__jack_urbanski__vibraphone-chord" 1.0 1.0 0.0 null null)
  (`KismetSystemLibrary.Delay` 0.5)
  (bind _outactors (`GameplayStatics.GetAllActorsOfClassWithTag` "/Script/Engine.CameraActor" "SafeOpeningCamera"))
  (`PlayerController.SetViewTargetWithBlend` (`GameplayStatics.GetPlayerController` 0) (`|GetArrayItem` _outactors) 0.0 "VTBlend_Linear" 0.0 false)
  (bind _foundwidgets (`WidgetBlueprintLibrary.GetAllWidgetsOfClass` "/Game/StarvingSeagulls/UI/LevelUI/FlapperRoomClickables.FlapperRoomClickables_C" false))
  (`/Game/StarvingSeagulls/UI/LevelUI/FlapperRoomClickables.SetBackButtonHidden` (`|GetArrayItem` _foundwidgets))
  (bind _foundwidgets_2 (`WidgetBlueprintLibrary.GetAllWidgetsOfClass` "/Game/StarvingSeagulls/UI/LevelUI/InGameHUD.InGameHUD_C" false))
  (`/Game/StarvingSeagulls/UI/LevelUI/InGameHUD.SetDiaryHidden` (`|GetArrayItem` _foundwidgets_2))
  (bind _outactors_2 (`GameplayStatics.GetAllActorsOfClass` "/Game/StarvingSeagulls/Blueprints/MediaManager/BP_MediaManager.BP_MediaManager_C"))
  (`/Game/StarvingSeagulls/Blueprints/MediaManager/BP_MediaManager.PlaySafeOpening` (`|GetArrayItem` _outactors_2))
  (`KismetSystemLibrary.Delay` 1.0)
  (`GameplayStatics.PlaySound2D` "/Game/StarvingSeagulls/Blueprints/Flappers-Room/FlapperSounds/399117__fastson__bultklick_01.399117__fastson__bultklick_01" 1.0 1.0 0.0 null null)
  (`KismetSystemLibrary.Delay` 0.5)
  (`GameplayStatics.PlaySound2D` "/Game/StarvingSeagulls/Blueprints/Flappers-Room/FlapperSounds/399117__fastson__bultklick_01.399117__fastson__bultklick_01" 1.0 1.0 0.0 null null)
  (`KismetSystemLibrary.Delay` 3.0)
  (bind _outactors_3 (`GameplayStatics.GetAllActorsOfClassWithTag` "/Script/Engine.CameraActor" "OccultBookCamera"))
  (`PlayerController.SetViewTargetWithBlend` (`GameplayStatics.GetPlayerController` 0) (`|GetArrayItem` _outactors_3) 0.0 "VTBlend_Linear" 0.0 false)
  (`KismetSystemLibrary.Delay` 6.0)
  (`GameplayStatics.OpenLevel` "EndGameLevel"))

(event `self.SecondDown.OnClicked`
  (params (TouchedComponent :type "PrimitiveComponent Object Reference") (ButtonPressed :type "Key Structure"))
  (bind _secondlock (`self.SecondLock`))
  (`GameplayStatics.PlaySound2D` "/Game/StarvingSeagulls/Blueprints/Flappers-Room/FlapperSounds/41506__digifishmusic__knife_sharpen_click.41506__digifishmusic__knife_sharpen_click" 1.0 1.0 0.0 null null)
  (if (> (`self.SecondLockValue`) 0)
    (`self.DecreaseValue` _secondlock)
    (goto _label)
    (else
      (`self.SetValueEleven` _secondlock)
      (goto _label))))

(event `self.ThirdUp.OnClicked`
  (params (TouchedComponent :type "PrimitiveComponent Object Reference") (ButtonPressed :type "Key Structure"))
  (bind _thirdlock (`self.ThirdLock`))
  (`GameplayStatics.PlaySound2D` "/Game/StarvingSeagulls/Blueprints/Flappers-Room/FlapperSounds/41506__digifishmusic__knife_sharpen_click.41506__digifishmusic__knife_sharpen_click" 1.0 1.0 0.0 null null)
  (if (< (`self.ThirdLockValue`) 11)
    (`self.IncreaseValue` _thirdlock)
    (goto _label)
    (else
      (`self.SetValueZero` _thirdlock)
      (goto _label))))

(event `self.ThirdDown.OnClicked`
  (params (TouchedComponent :type "PrimitiveComponent Object Reference") (ButtonPressed :type "Key Structure"))
  (bind _thirdlock (`self.ThirdLock`))
  (`GameplayStatics.PlaySound2D` "/Game/StarvingSeagulls/Blueprints/Flappers-Room/FlapperSounds/41506__digifishmusic__knife_sharpen_click.41506__digifishmusic__knife_sharpen_click" 1.0 1.0 0.0 null null)
  (if (> (`self.ThirdLockValue`) 0)
    (`self.DecreaseValue` _thirdlock)
    (goto _label)
    (else
      (`self.SetValueEleven` _thirdlock)
      (goto _label))))

(fn `DecreaseValue`
  (params (Lock :type "PaperSpriteComponent Object Reference"))
  (if (== Lock (`self.FirstLock`))
    (set `self.FirstLockValue` (- (`self.FirstLockValue`) 1))
    (`PaperSpriteComponent.SetSprite` (`self.FirstLock`) (`|GetArrayItem` (`self.NumberSprites`) (`self.FirstLockValue`)))
    (elif (== Lock (`self.SecondLock`))
      (set `self.SecondLockValue` (- (`self.SecondLockValue`) 1))
      (`PaperSpriteComponent.SetSprite` (`self.SecondLock`) (`|GetArrayItem` (`self.NumberSprites`) (`self.SecondLockValue`)))
      (elif (== Lock (`self.ThirdLock`))
        (set `self.ThirdLockValue` (- (`self.ThirdLockValue`) 1))
        (`PaperSpriteComponent.SetSprite` (`self.ThirdLock`) (`|GetArrayItem` (`self.NumberSprites`) (`self.ThirdLockValue`)))
        (else
          (`KismetSystemLibrary.PrintString` "If you're seeing this something has gone VERY wrong"))))))

(fn `IncreaseValue`
  (params (Lock :type "PaperSpriteComponent Object Reference"))
  (if (== Lock (`self.FirstLock`))
    (set `self.FirstLockValue` (+ (`self.FirstLockValue`) 1))
    (`PaperSpriteComponent.SetSprite` (`self.FirstLock`) (`|GetArrayItem` (`self.NumberSprites`) (`self.FirstLockValue`)))
    (elif (== Lock (`self.SecondLock`))
      (set `self.SecondLockValue` (+ (`self.SecondLockValue`) 1))
      (`PaperSpriteComponent.SetSprite` (`self.SecondLock`) (`|GetArrayItem` (`self.NumberSprites`) (`self.SecondLockValue`)))
      (elif (== Lock (`self.ThirdLock`))
        (set `self.ThirdLockValue` (+ (`self.ThirdLockValue`) 1))
        (`PaperSpriteComponent.SetSprite` (`self.ThirdLock`) (`|GetArrayItem` (`self.NumberSprites`) (`self.ThirdLockValue`)))
        (else
          (`KismetSystemLibrary.PrintString` "If you're seeing this something has gone VERY wrong"))))))

(fn `SetValueEleven`
  (params (Lock :type "PaperSpriteComponent Object Reference"))
  (if (== Lock (`self.FirstLock`))
    (set `self.FirstLockValue` 11)
    (`PaperSpriteComponent.SetSprite` (`self.FirstLock`) (`|GetArrayItem` (`self.NumberSprites`) (`self.FirstLockValue`)))
    (elif (== Lock (`self.SecondLock`))
      (set `self.SecondLockValue` 11)
      (`PaperSpriteComponent.SetSprite` (`self.SecondLock`) (`|GetArrayItem` (`self.NumberSprites`) (`self.SecondLockValue`)))
      (elif (== Lock (`self.ThirdLock`))
        (set `self.ThirdLockValue` 11)
        (`PaperSpriteComponent.SetSprite` (`self.ThirdLock`) (`|GetArrayItem` (`self.NumberSprites`) (`self.ThirdLockValue`)))
        (else
          (`KismetSystemLibrary.PrintString` "If you're seeing this something has gone VERY wrong"))))))

(fn `SetValueZero`
  (params (Lock :type "PaperSpriteComponent Object Reference"))
  (if (== Lock (`self.FirstLock`))
    (set `self.FirstLockValue` 0)
    (`PaperSpriteComponent.SetSprite` (`self.FirstLock`) (`|GetArrayItem` (`self.NumberSprites`) (`self.FirstLockValue`)))
    (elif (== Lock (`self.SecondLock`))
      (set `self.SecondLockValue` 0)
      (`PaperSpriteComponent.SetSprite` (`self.SecondLock`) (`|GetArrayItem` (`self.NumberSprites`) (`self.SecondLockValue`)))
      (elif (== Lock (`self.ThirdLock`))
        (set `self.ThirdLockValue` 0)
        (`PaperSpriteComponent.SetSprite` (`self.ThirdLock`) (`|GetArrayItem` (`self.NumberSprites`) (`self.ThirdLockValue`)))
        (else
          (`KismetSystemLibrary.PrintString` "If you're seeing this something has gone VERY wrong"))))))

(fn `SolutionChecker`
  (bind _currentvalues (`self.CurrentValues`))
  (`KismetArrayLibrary.Array_Clear` _currentvalues)
  (`KismetArrayLibrary.Array_Add` _currentvalues (`self.FirstLockValue`))
  (`KismetArrayLibrary.Array_Add` _currentvalues (`self.SecondLockValue`))
  (`KismetArrayLibrary.Array_Add` _currentvalues (`self.ThirdLockValue`))
  (if (`KismetArrayLibrary.Array_Identical` (`self.Solution`) _currentvalues)
    (`self.SafePuzzleComplete`)))

(fn `UserConstructionScript`
  (`PaperSpriteComponent.SetSprite` (`self.FirstLock`) (`|GetArrayItem` (`self.NumberSprites`) (`self.FirstLockValue`)))
  (`PaperSpriteComponent.SetSprite` (`self.SecondLock`) (`|GetArrayItem` (`self.NumberSprites`) (`self.SecondLockValue`)))
  (`PaperSpriteComponent.SetSprite` (`self.ThirdLock`) (`|GetArrayItem` (`self.NumberSprites`) (`self.ThirdLockValue`))))