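; Media manager actor that prepares the game's video playback for a fish background, a safe animation and a book animation.
; On BeginPlay it opens each media source on its own Media Player.
; PlaySafeOpening turns off looping on the safe player, rewinds it and plays the opening from the start.
; The fish and book players have no playback controls here beyond opening their sources.
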(event `self.ReceiveBeginPlay`
  (`MediaPlayer.OpenSource` (`self.FishMediaPlayer`) "/Game/StarvingSeagulls/Art-Assets/Animations/Fish_Background_for_Window/fish_background.fish_background")
  (`MediaPlayer.OpenSource` (`self.SafeMediaPlayer`) "/Game/Movies/safeAnimation.safeAnimation")
  (`MediaPlayer.OpenSource` (`self.BookMediaPlayer`) "/Game/Movies/bookAnimation.bookAnimation"))

(fn `PlaySafeOpening`
  (bind _safemediaplayer (`self.SafeMediaPlayer`))
  (`MediaPlayer.SetLooping` _safemediaplayer false)
  (`MediaPlayer.Rewind` _safemediaplayer)
  (`MediaPlayer.Play` _safemediaplayer))

(fn `UserConstructionScript`)